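; AC_LandingSmokeTest is a debug actor component that smoke-tests the landing EQS query against the ThreatFieldSubsystem.
; EQSSmokeTest registers an area center just ahead of the owner with its Ability System Component and an ActivationId.
; It runs LandingQuery for all matches, passing ActivationId as a named param to link the query to that area.
; The finish callback draws debug spheres at result locations and prints the point count, or reports failure.
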(fn `EQS_SmokeTest`
  (locals (Owner :type "Actor Object Reference") (ASC :type "AbilitySystemComponent Object Reference") (Center :type "Vector Structure") (Wrapper :type "EnvQueryInstanceBlueprintWrapper Object Reference"))
  (bind _owner (`local.Owner`))
  (bind _output_get (set `local.Owner` (`self.GetOwner`)))
  (set `local.ASC` (`AbilitySystemBlueprintLibrary.GetAbilitySystemComponent` _output_get))
  (set `local.Center` (+ (`Actor.K2_GetActorLocation` _owner) (* (`Actor.GetActorForwardVector` _owner) 50.0)))
  (`ThreatFieldSubsystem.RegisterAreaCenter` (subsystem `ThreatFieldSubsystem`) (`local.ASC`) (`self.ActivationId`) (`local.Center`) (`self.AreaRadius`) 0.0)
  (bind _returnvalue (`EnvQueryManager.RunEQSQuery` (`self.LandingQuery`) (`local.Owner`) "AllMatching" "/Script/AIModule.EnvQueryInstanceBlueprintWrapper"))
  (bind _output_get_2 (set `local.Wrapper` _returnvalue))
  (`EnvQueryInstanceBlueprintWrapper.SetNamedParam` _output_get_2 "ActivationId" (`KismetMathLibrary.Conv_IntToDouble` (`self.ActivationId`)))
  (add `EnvQueryInstanceBlueprintWrapper.OnQueryFinishedEvent` (`local.Wrapper`) (`|CreateDelegate` :!event `OnEQSFinished`)))

(fn `OnEQSFinished`
  (params (QueryInstance :type "EnvQueryInstanceBlueprintWrapper Object Reference") (QueryStatus :type "EEnvQueryStatus Enum" :default "Processing"))
  (if (`|EnumInequality` QueryStatus "Success")
    (`KismetSystemLibrary.PrintString` "EQS Failed" true true (struct :`R` 0.088542 :`B` 0.003564 :`A` 1.0))
    (return)
    (else
      (bind _resultlocations (`EnvQueryInstanceBlueprintWrapper.GetQueryResultsAsLocations` QueryInstance))
      (for _array_element _resultlocations
        (`KismetSystemLibrary.DrawDebugSphere` _array_element 35.0 12 (struct :`R` 0.983123 :`B` 1.0 :`A` 1.0) 10.0))
      (`KismetSystemLibrary.PrintString` (`KismetStringLibrary.Concat_StrStr` "EQS Success: " (`KismetStringLibrary.Conv_IntToString` (`KismetArrayLibrary.Array_Length` _resultlocations)) " points.")))))