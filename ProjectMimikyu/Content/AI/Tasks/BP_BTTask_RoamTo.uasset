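; Behavior tree task that makes a BP_Lucario pawn roam to a random point around its spawn location.
; It sets a fixed walk speed, picks a navigable point within a radius of the SpawnLocation blackboard value and stores it in TargetLocation.
; An AI MoveTo heads to that point and finishes the task as success or failure, with debug prints along the way.
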(event `self.ReceiveExecuteAI`
  (params (OwnerController :type "AIController Object Reference") (ControlledPawn :type "Pawn Object Reference"))
  (bind _asbp_lucario (cast `/Game/Blueprints/Characters/Pokemon/Lucario/BP_Lucario` ControlledPawn))
  (bind _charactermovement (`Character.CharacterMovement` _asbp_lucario)
    (:`then`
      (set `CharacterMovementComponent.MaxWalkSpeed` 250.0 _charactermovement)
      (bind _randomlocation (`NavigationSystemV1.K2_GetRandomLocationInNavigableRadius` (`BTFunctionLibrary.GetBlackboardValueAsVector` (`self.SpawnLocation`)) 500.0 null null))
      (`BTFunctionLibrary.SetBlackboardValueAsVector` (`self.TargetLocation`) _randomlocation)
      (bind _movementresult (`|AIMoveTo` null _randomlocation null)
        (:`then`
          (bind _output_get (set `self.Movement Result` _movementresult))
          (`KismetSystemLibrary.PrintString` "why isn't this working?")
          (`KismetSystemLibrary.PrintString` (`KismetStringLibrary.Concat_StrStr` "Movement Result is " (`|GetEnumeratorNameAsString` _output_get))))
        (:`OnSuccess`
          (`KismetSystemLibrary.PrintString` "succeeded")
          (`self.FinishExecute` true))
        (:`OnFail`
          (`KismetSystemLibrary.PrintString` "failing")
          (`self.FinishExecute` false))))
    (:`else`)))