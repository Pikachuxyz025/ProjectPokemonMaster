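; Base Gameplay Ability for Pokemon melee moves, covering command registration, target approach and hit resolution.
; After commit, trainer-owned Pokemon acknowledge commands, delayed with a blue material unless sequenced, then CombatApproachTask closes range and starts anticipation.
; StartActive resolves a contact sphere and applies impact-adjusted damage to live actors inside.
; An airborne miss can enter whiff recovery; debug prints and an optional presentation-preview branch support testing.
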(event `self.RegisterCommand`
  (bind _movetimingsequence_commanddelay (break `MoveTiming` (`self.MoveTimingSequence`)))
  (if (`Pokemon_Parent.HasTrainer` (`self.Pokemon`))
    (if (`self.IsSequencedExecution`)
      (`KismetSystemLibrary.PrintString` "Command Acknowledged" true true (struct :`R` 0.948237 :`G` 1.0 :`A` 1.0) :!label _label)
      (`self.ReturnToOriginalMaterial`)
      (`self.MoveToTarget`)
      (else
        (`AbilityTask_WaitDelay.WaitDelay` _movetimingsequence_commanddelay
          (:`then`
            (`KismetSystemLibrary.PrintString` "Registering Command")
            (`PrimitiveComponent.SetMaterial` (`self.PokemonMesh`) 0 "/Game/Assets/Materials/M_Blue.M_Blue"))
          (:`OnFinish`
            (goto _label)))))
    (else
      (`self.MoveToTarget`))))

(event `self.K2_ActivateAbility`
  (bind _returnvalue (`self.CommitPokemonMove`))
  (if _returnvalue
    (`self.GetCurrentPokemonMeshAndMaterial`)
    (`self.RegisterCommand`)
    (else
      (`self.K2_EndAbility`))))

(event `MoveToTarget`
  (bind _returnvalue (message `PokemonCombatInterface.GetCombatTarget` (`self.GetAvatarActorFromActorInfo`)))
  (`AT_CombatApproach.CreateCombatApproachTask` "Approaching Target" _returnvalue (`self.IdealRange`) (`self.SpeedMultiplier`)
    (:`OnReachedRange`
      (`self.StartAnticipation`))
    (:`OnFailed`
      (`KismetSystemLibrary.PrintString` "Pokemon failed to reach or move to target")
      (`self.K2_EndAbility`))))

(event `self.StartActive`
  (bind _returnvalue (`self.GetAvatarActorFromActorInfo`))
  (bind (_outcenter _outradius _returnvalue_2) (`PokemonMeleeContactLibrary.ResolveMeleeContactSphere` _returnvalue (`self.MeleeContact`) true))
  (if _returnvalue_2
    (bind _outoverlappingactors (`PokemonAbilitySystemLibrary.GetLivePlayersWithinRadius` _returnvalue (`|MakeArray` _returnvalue) _outradius _outcenter))
    (bind _returnvalue_3 (`KismetArrayLibrary.Array_Length` _outoverlappingactors))
    (if (> _returnvalue_3 0)
      (`KismetSystemLibrary.PrintString` (`KismetStringLibrary.Concat_StrStr` "There Are " (`KismetStringLibrary.Conv_IntToString` _returnvalue_3) "hit Pokemon"))
      (for _array_element _outoverlappingactors
        (bind (_outimpactresolution _returnvalue_4) (`self.ResolveImpactAndModifyDamageParams` _array_element (`self.MakeDamageEffectParamsFromClassDefaults` _array_element)))
        (`PokemonAbilitySystemLibrary.ApplyDamageEffect` _returnvalue_4)
        (if (`self.bEnablePresentationBranchTest`)
          (`self.PreviewConfirmedOutcome` "Hit")))
      (bind _returnvalue_5 (`self.ConfirmAirborneMissAtActiveWindowEnd` :!label _label_2))
      (if _returnvalue_5
        (bind _returnvalue_6 (`self.BeginAirborneWhiffRecovery`))
        (if (not _returnvalue_6)
          (if (not (`self.bEnablePresentationBranchTest`)) :!label _label_3
            (`self.K2_EndAbility`)))
        (else
          (goto _label_3)))
      (else
        (`KismetSystemLibrary.PrintString` "There are no hit targets")
        (if (`self.bEnablePresentationBranchTest`)
          (`|ExecutionSequence`
            (:`then_0`
              (goto _label_2))
            (:`then_1`
              (`self.PreviewConfirmedOutcome` "Miss")))
          (else
            (goto _label_2)))))
    (else
      (`KismetSystemLibrary.PrintString` "Invalid melee contact configuration")
      (`self.K2_EndAbility`))))

(event `self.K2_OnEndAbility`
  (params (bWasCancelled :type Boolean))
  (`parent.K2_OnEndAbility` bWasCancelled))

(fn `GetCurrentMaterialInstance`
  (returns (Mesh :type "SkeletalMeshComponent Object Reference")))