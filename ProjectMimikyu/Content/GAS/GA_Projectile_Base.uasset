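; Base Gameplay Ability for a Pokémon projectile move, run in timed command, anticipation and active phases.
; After committing, it waits a command delay only if the Pokémon has a trainer, then flashes the mesh material during anticipation and restores it.
; The active phase takes target data and spawns a projectile from the projectile socket toward a hit or end point.
; It ends after a fixed delay, notifying the Pokémon that the attack ended.
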(event `self.K2_ActivateAbility`
  (bind _returnvalue (`self.CommitPokemonMove`))
  (if _returnvalue
    (`self.SetupPokemon`)
    (`self.RegisterCommand`)
    (else
      (`self.K2_EndAbility`))))

(event `StartAnticipation`
  (bind (_movetimingsequence_commanddelay _movetimingsequence_anticipationduration) (break `MoveTiming` (`self.MoveTimingSequence`)))
  (`PrimitiveComponent.SetMaterial` (`self.PokemonMesh`) 0 "/Game/Assets/Materials/M_AnticpationFlash.M_AnticpationFlash")
  (`AbilityTask_WaitDelay.WaitDelay` _movetimingsequence_anticipationduration
    (:`then`
      (`KismetSystemLibrary.PrintString` "Anticipation Phase" true true (struct :`R` 1.0 :`G` 0.516844 :`B` 0.02598 :`A` 1.0)))
    (:`OnFinish`
      (for (_array_element _array_index) (`self.CurrentMaterialInstance`)
        (`PrimitiveComponent.SetMaterial` (`self.PokemonMesh`) _array_index _array_element))
      (`self.StartActive`))))

(event `StartActive`
  (bind _returnvalue (`BlueprintGameplayTagLibrary.MakeLiteralGameplayTag` (struct :`TagName` "CombatSocket.Projectile")))
  (bind (_asynctaskproxy _datahandle) (`AT_TargetDataLocation.CreateTargetDataLocation`)
    (:`ValidData`
      (if (`AbilitySystemBlueprintLibrary.TargetDataHasHitResult` _datahandle)
        (bind _returnvalue_2 (`AbilitySystemBlueprintLibrary.GetActorsFromTargetData` _datahandle))
        (if (not (> (`KismetArrayLibrary.Array_Length` _returnvalue_2) 1))
          (`self.SpawnProjectile` (`.Location` (`GameplayStatics.BreakHitResult` (`AbilitySystemBlueprintLibrary.GetHitResultFromTargetData` _datahandle))) _returnvalue (`|GetArrayItem` _returnvalue_2))
          (`KismetSystemLibrary.Delay` 2.0 :!label _label)
          (`self.K2_EndAbility`))
        (else
          (`self.SpawnProjectile` (`AbilitySystemBlueprintLibrary.GetTargetDataEndPoint` _datahandle) _returnvalue)
          (goto _label))))))

(event `self.K2_OnEndAbility`
  (params (bWasCancelled :type Boolean))
  (bind _pokemon (`self.Pokemon`)
    (:`then`
      (`Pokemon_Parent.AttackEnded` _pokemon))
    (:`else`
      (bind _aspokemon_parent (cast `Pokemon_Parent` (`self.GetAvatarActorFromActorInfo`)))
      (bind _output_get (set `self.Pokemon` _aspokemon_parent))
      (`Pokemon_Parent.AttackEnded` _output_get))))

(event `RegisterCommand`
  (bind _movetimingsequence_commanddelay (break `MoveTiming` (`self.MoveTimingSequence`)))
  (if (`Pokemon_Parent.HasTrainer` (`self.Pokemon`))
    (`AbilityTask_WaitDelay.WaitDelay` _movetimingsequence_commanddelay
      (:`then`
        (`KismetSystemLibrary.PrintString` "Registering Command")
        (`PrimitiveComponent.SetMaterial` (`self.PokemonMesh`) 0 "/Game/Assets/Materials/M_Blue.M_Blue"))
      (:`OnFinish`
        (`KismetSystemLibrary.PrintString` "Command Acknowledged" true true (struct :`R` 0.948237 :`G` 1.0 :`A` 1.0))
        (`self.StartAnticipation`)))
    (else
      (`self.StartAnticipation`))))

(fn `SetupPokemon`
  (bind _aspokemon_parent (cast `Pokemon_Parent` (`self.GetAvatarActorFromActorInfo`)))
  (bind _output_get (set `self.Pokemon` _aspokemon_parent))
  (bind _mesh (`Character.Mesh` _output_get))
  (set `self.CurrentMaterialInstance` (`MeshComponent.GetMaterials` _mesh))
  (set `self.PokemonMesh` _mesh))