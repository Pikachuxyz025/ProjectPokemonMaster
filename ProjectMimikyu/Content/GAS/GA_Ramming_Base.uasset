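; Base ramming Gameplay Ability that dashes the avatar at its combat target and damages what it strikes.
; A constant-force root motion task drives the dash while a tick task sphere-traces for pawns.
; The first blocking hit with an ability system interface receives the class-default damage effect, ending both tasks and the ability, as does dash completion.
; Older capsule-collision, launch and line-trace approaches remain as unconnected nodes.
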(event `ActivateAbilitie`
  (bind _returnvalue (`self.GetAvatarActorFromActorInfo`))
  (bind _returnvalue_2 (`Actor.K2_GetActorLocation` _returnvalue))
  (bind _tocombattarget (`self.Get Direction To Combat Target` (`self.GetAvatarActorFromActorInfo`)))
  (`AbilityTask_ApplyRootMotionConstantForce.ApplyRootMotionConstantForce` "DashEvent" _tocombattarget (`self.DashSpeed`) (`self.DashDuration`) false null "MaintainLastRootMotionVelocity"
    (:`then`
      (`AT_TickTask.CreateTickTaskNode` "RamTick"
        (:`OnTick`
          (bind _outhit (`KismetSystemLibrary.SphereTraceSingleForObjects` _returnvalue_2 (* (+ _returnvalue_2 (`Actor.GetActorForwardVector` _returnvalue)) (`self.TraceRange`)) (`self.TraceRadius`) (`|MakeArray` "ObjectTypeQuery3" :!type "EObjectTypeQuery Enum") false (`|MakeArray` (`self.GetAvatarActorFromActorInfo`)) "ForDuration" true (struct :`R` 0.030746 :`G` 0.66444 :`B` 1.0 :`A` 1.0) (struct :`R` 0.135595 :`G` 1.0 :`A` 1.0)))
          (if (and (`GameplayStatics.BreakHitResult` _outhit) (`KismetSystemLibrary.DoesImplementInterface` (`.HitActor` (`GameplayStatics.BreakHitResult` _outhit)) "/Script/GameplayAbilities.AbilitySystemInterface"))
            (bind _output_get (set `self.DashHitActor` (`.HitActor` (`GameplayStatics.BreakHitResult` _outhit))))
            (`PokemonAbilitySystemLibrary.ApplyDamageEffect` (`self.MakeDamageEffectParamsFromClassDefaults` _output_get))
            (`self.EndTaskByInstanceName` "RamTick")
            (`self.EndTaskByInstanceName` "DashEvent")
            (`self.K2_EndAbility`)))))
    (:`OnFinish`
      (`KismetSystemLibrary.PrintString` "Ending Attack")
      (`self.EndTaskByInstanceName` "DashEvent")
      (`self.EndTaskByInstanceName` "RamTick")
      (`self.K2_EndAbility`))))

(event `self.K2_ActivateAbility`
  (`parent.K2_ActivateAbility`)
  (`KismetSystemLibrary.PrintString` "ramming")
  (`self.ActivateAbilitie`))

(event `OnComponentHit_Event`
  (params (HitComponent :type "PrimitiveComponent Object Reference") (OtherActor :type "Actor Object Reference") (OtherComp :type "PrimitiveComponent Object Reference") (NormalImpulse :type "Vector Structure") (Hit :type "HitResult Structure (by ref)"))
  (if (`KismetSystemLibrary.DoesImplementInterface` OtherActor "/Script/GameplayAbilities.AbilitySystemInterface")
    (`KismetSystemLibrary.PrintString` (`KismetStringLibrary.Concat_StrStr` "Hit Target: " (`KismetSystemLibrary.GetDisplayName` (stale `OnComponentBeginOverlap_Event` OtherActor))) true true (struct :`R` 0.583229 :`G` 1.0 :`A` 1.0) :!label _label)
    (`PokemonAbilitySystemLibrary.ApplyDamageEffect` (`self.MakeDamageEffectParamsFromClassDefaults` OtherActor))
    (else
      (`KismetSystemLibrary.PrintString` (`KismetStringLibrary.Concat_StrStr` "Hit But Incorrect Target: " (`KismetSystemLibrary.GetDisplayName` OtherActor)))))
  (`self.K2_EndAbility`))

(event `OnComponentBeginOverlap_Event`
  (params (OverlappedComponent :type "PrimitiveComponent Object Reference") (OtherActor :type "Actor Object Reference") (OtherComp :type "PrimitiveComponent Object Reference") (OtherBodyIndex :type Integer) (bFromSweep :type Boolean) (SweepResult :type "HitResult Structure (by ref)"))
  (goto _label))

(event `self.K2_OnEndAbility`
  (params (bWasCancelled :type Boolean))
  (`parent.K2_OnEndAbility` bWasCancelled))

(event `OnCharging_Event`
  (`KismetSystemLibrary.PrintString` "end attack")
  (`self.K2_EndAbility`))

(fn `Get Direction To Combat Target`
  (params (NewActor :type "Actor Object Reference"))
  (returns (ToCombatTarget :type "Vector Structure"))
  (bind _returnvalue (message `PokemonCombatInterface.GetCombatTarget` NewActor))
  (return (`KismetMathLibrary.Normal` (- (`Actor.K2_GetActorLocation` _returnvalue) (`Actor.K2_GetActorLocation` NewActor)))))