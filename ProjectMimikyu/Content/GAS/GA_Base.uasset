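; Base Gameplay Ability for Pokemon moves that sequences command, anticipation and active phases.
; After committing, it caches the mesh and materials, waits out a command delay only for trainer-owned Pokemon, then runs anticipation.
; Timed ability tasks drive debug prints and material swaps, restoring materials before StartActive, an empty hook presumably for child moves.
; Ending the ability calls AttackEnded on the Pokemon.
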(event `self.K2_ActivateAbility`
  (bind _returnvalue (`self.CommitPokemonMove`))
  (if _returnvalue
    (`self.GetCurrentPokemonMeshAndMaterial`)
    (`self.RegisterCommand`)
    (else
      (`self.K2_EndAbility`))))

(event `self.K2_OnEndAbility`
  (params (bWasCancelled :type Boolean))
  (bind _pokemon (`self.Pokemon`)
    (:`then`
      (`Pokemon_Parent.AttackEnded` _pokemon))
    (:`else`
      (bind _aspokemon_parent (cast `Pokemon_Parent` (`self.GetAvatarActorFromActorInfo`)))
      (`Pokemon_Parent.AttackEnded` _aspokemon_parent))))

(event `StartAnticipation`
  (bind (_movetimingsequence_commanddelay _movetimingsequence_anticipationduration) (break `MoveTiming` (`self.MoveTimingSequence`)))
  (`PrimitiveComponent.SetMaterial` (`self.PokemonMesh`) 0 "/Game/Assets/Materials/M_AnticpationFlash.M_AnticpationFlash")
  (`AbilityTask_WaitDelay.WaitDelay` _movetimingsequence_anticipationduration
    (:`then`
      (`KismetSystemLibrary.PrintString` "Anticipation Phase" true true (struct :`R` 1.0 :`G` 0.516844 :`B` 0.02598 :`A` 1.0)))
    (:`OnFinish`
      (`self.ReturnToOriginalMaterial`)
      (`self.StartActive`))))

(event `StartActive`)

(event `RegisterCommand`
  (bind _movetimingsequence_commanddelay (break `MoveTiming` (`self.MoveTimingSequence`)))
  (if (`Pokemon_Parent.HasTrainer` (`self.Pokemon`))
    (`AbilityTask_WaitDelay.WaitDelay` _movetimingsequence_commanddelay
      (:`then`
        (`KismetSystemLibrary.PrintString` "Registering Command")
        (`PrimitiveComponent.SetMaterial` (`self.PokemonMesh`) 0 "/Game/Assets/Materials/M_Blue.M_Blue"))
      (:`OnFinish`
        (`KismetSystemLibrary.PrintString` "Command Acknowledged" true true (struct :`R` 0.948237 :`G` 1.0 :`A` 1.0))
        (`self.StartAnticipation`)))
    (else
      (`self.StartAnticipation`))))

(fn `GetCurrentPokemonMeshAndMaterial`
  (bind _aspokemon_parent (cast `Pokemon_Parent` (`self.GetAvatarActorFromActorInfo`)))
  (bind _output_get (set `self.Pokemon` _aspokemon_parent))
  (bind _mesh (`Character.Mesh` _output_get))
  (set `self.CurrentMaterialInstance` (`MeshComponent.GetMaterials` _mesh))
  (set `self.PokemonMesh` _mesh))

(fn `ReturnToOriginalMaterial`
  (for (_array_element _array_index) (`self.CurrentMaterialInstance`)
    (`PrimitiveComponent.SetMaterial` (`self.PokemonMesh`) _array_index _array_element))
  (return))

(fn `ShowPokemonMove`
  (bind _aspokemon_parent (cast `Pokemon_Parent` (`self.GetAvatarActorFromActorInfo`)))
  (bind _output_get (set `self.Pokemon` _aspokemon_parent))
  (`/Engine/EditorBlueprintResources/StandardMacros.IsValid` (`PokemonCommandComponent.GetActiveMove` (`Pokemon_Parent.CommandComponent` _output_get))
    (:`Is Not Valid`
      (`self.K2_EndAbility`))))