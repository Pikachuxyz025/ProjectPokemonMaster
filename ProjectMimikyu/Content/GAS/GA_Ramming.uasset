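; Gameplay Ability for a Pokemon ramming attack that damages what the Pokemon runs into, then ends.
; On activation it binds capsule hits and starts a tick task that traces a short line forward.
; A trace or capsule hit causes damage, with the capsule path also calling the Pokemon's OnBoxHit.
; The OnCharging delegate or a timeout also ends the ram, reusing the hit path if a hit component is valid.
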(event `self.K2_ActivateAbility`
  (bind _pokemon (`self.Pokemon`))
  (bind _returnvalue (`Actor.K2_GetActorLocation` _pokemon))
  (`parent.K2_ActivateAbility`)
  (`KismetSystemLibrary.PrintString` "ramming")
  (add `PrimitiveComponent.OnComponentHit` (`Character.CapsuleComponent` (`self.Pokemon`)) (delegate `OnComponentHit_Event`))
  (`AT_TickTask.CreateTickTaskNode` "RamTick"
    (:`then`
      (add `Pokemon_Parent.OnCharging` (`self.Pokemon`) (delegate `OnCharging_Event`))
      (`KismetSystemLibrary.K2_SetTimerDelegate` (delegate `OnCharging_Event`) 5.0))
    (:`OnTick`
      (bind _outhit (`KismetSystemLibrary.LineTraceSingle` _returnvalue (+ _returnvalue (* (`Actor.GetActorForwardVector` _pokemon) 75.0)) "TraceTypeQuery1"))
      (`/Engine/EditorBlueprintResources/StandardMacros.IsValid` (`.HitActor` (`GameplayStatics.BreakHitResult` _outhit))
        (:`Is Valid`
          (`self.CauseDamage` (`.HitActor` (`GameplayStatics.BreakHitResult` _outhit)))
          (`self.EndTaskByInstanceName` "RamTick")
          (`self.K2_EndAbility`))))))

(event `self.K2_OnEndAbility`
  (params (bWasCancelled :type Boolean))
  (`parent.K2_OnEndAbility` bWasCancelled))

(event `OnComponentHit_Event`
  (params (HitComponent :type "PrimitiveComponent Object Reference") (OtherActor :type "Actor Object Reference") (OtherComp :type "PrimitiveComponent Object Reference") (NormalImpulse :type "Vector Structure") (Hit :type "HitResult Structure (by ref)"))
  (`self.CauseDamage` OtherActor :!label _label)
  (`Pokemon_Parent.OnBoxHit` (`self.Pokemon`) HitComponent OtherActor OtherComp NormalImpulse Hit)
  (`self.EndTaskByInstanceName` "RamTick")
  (`self.K2_EndAbility`))

(event `OnCharging_Event`
  (`KismetSystemLibrary.PrintString` "end attack")
  (if (`KismetSystemLibrary.IsValid` (stale `OnComponentHit_Event` HitComponent))
    (goto _label)
    (else
      (clear `Pokemon_Parent.OnCharging` (`self.Pokemon`))
      (`self.EndTaskByInstanceName` "RamTick")
      (`self.K2_EndAbility`))))