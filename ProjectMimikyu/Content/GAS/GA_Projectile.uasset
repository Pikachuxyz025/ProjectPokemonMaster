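; Gameplay Ability that fires a projectile attack for the avatar Pokemon.
; On activation it caches the Pokemon and prints the active move's name, calling EndAbility if no move is valid.
; A target-data task supplies the location, using the hit result or the end point as fallback, for SpawnProjectile.
; The ability ends after a short delay, and its end event calls AttackEnded on the Pokemon.
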(event `self.K2_ActivateAbility`
  (`self.ShowPokemonMove`)
  (bind (_asynctaskproxy _datahandle) (`AT_TargetDataLocation.CreateTargetDataLocation`)
    (:`ValidData`
      (if (`AbilitySystemBlueprintLibrary.TargetDataHasHitResult` _datahandle)
        (`self.SpawnProjectile` (`.Location` (`GameplayStatics.BreakHitResult` (`AbilitySystemBlueprintLibrary.GetHitResultFromTargetData` _datahandle))))
        (else
          (`self.SpawnProjectile` (`AbilitySystemBlueprintLibrary.GetTargetDataEndPoint` _datahandle))))
      (`KismetSystemLibrary.Delay` 2.0)
      (`self.K2_EndAbility`))))

(event `self.K2_OnEndAbility`
  (params (bWasCancelled :type Boolean))
  (`Pokemon_Parent.AttackEnded` (`self.Pokemon`)))

(fn `ShowPokemonMove`
  (bind _aspokemon_parent (cast `Pokemon_Parent` (`self.GetAvatarActorFromActorInfo`)))
  (bind _output_get (set `self.Pokemon` _aspokemon_parent))
  (bind _activepokemonmove (`Pokemon_Parent.ActivePokemonMove` _output_get))
  (`/Engine/EditorBlueprintResources/StandardMacros.IsValid` _activepokemonmove
    (:`Is Valid`
      (`KismetSystemLibrary.PrintString` (`KismetTextLibrary.Conv_TextToString` (`PokemonMoveDataAsset.MoveName` _activepokemonmove)) true true (struct :`R` 1.0 :`G` 0.112648 :`B` 0.082801 :`A` 1.0)))
    (:`Is Not Valid`
      (`self.K2_EndAbility`))))